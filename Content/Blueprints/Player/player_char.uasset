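; Player character Blueprint that turns input into walking, strafing, jumping, crouching and camera look.
; Movement axes add input along the actor's forward and right vectors, while look axes drive controller yaw and pitch.
; Crouch and sprint are hold actions.
; Sprint sets a flag and a multiplier that scales only the forward/back input vector, leaving strafing and movement component speed settings untouched.
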(event Input|ActionEvents|InputActionJump
  (params (Key :type Key%20Structure :default "AnyKey"))
  (:Pressed
    (Character|Jump)))

(event Input|ActionEvents|InputActionCrouch
  (params (Key :type Key%20Structure :default "AnyKey"))
  (:Pressed
    (Character|Crouch))
  (:Released
    (Character|UnCrouch)))

(event Input|ActionEvents|InputActionSprint
  (params (Key :type Key%20Structure :default "AnyKey"))
  (:Pressed
    (Variables|Default|SetisSprinting true)
    (Variables|Default|SetsprintMultiplyer 2.0))
  (:Released
    (Variables|Default|SetisSprinting false)
    (Variables|Default|SetsprintMultiplyer 1.0)))

(event Input|AxisEvents|InputAxisMoveForward
  (params (AxisValue :type Float%20%28single-precision%29))
  ;[1 1 1] Movement
  (Pawn|Input|AddMovementInput (* (Transformation|GetActorForwardVector) (Variables|Default|GetsprintMultiplyer)) AxisValue false))

(event Input|AxisEvents|InputAxisLookUP
  (params (AxisValue :type Float%20%28single-precision%29))
  ;[1 1 1] Looking
  (Pawn|Input|AddControllerPitchInput AxisValue))

(event Input|AxisEvents|InputAxisMoveRight
  (params (AxisValue :type Float%20%28single-precision%29))
  ;[1 1 1] Movement
  (Pawn|Input|AddMovementInput (Transformation|GetActorRightVector) AxisValue false))

(event Input|AxisEvents|InputAxisLookTurn
  (params (AxisValue :type Float%20%28single-precision%29))
  ;[1 1 1] Looking
  (Pawn|Input|AddControllerYawInput AxisValue))

(fn ConstructionScript)